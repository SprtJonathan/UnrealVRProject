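; BP_Enemy_Master is a human enemy character Blueprint, named as a master class, that handles taking damage and dying.
; AnyDamage subtracts incoming damage from Health and calls Death once the value drops below zero.
; Death destroys the capsule, ragdolls the mesh through physics simulation, plays DeathSound at the mesh location, then destroys the actor after a delay.
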(event `Death`
  (bind _mesh (`self.Mesh`))
  (`ActorComponent.K2_DestroyComponent` (`self.CapsuleComponent`))
  (`PrimitiveComponent.SetSimulatePhysics` _mesh true)
  (`GameplayStatics.PlaySoundAtLocation` (`self.DeathSound`) (`SceneComponent.K2_GetComponentLocation` _mesh) (struct) 1.0 1.0 0.0 null null null null)
  (`KismetSystemLibrary.Delay` 10.0)
  (`self.K2_DestroyActor`))

(event `self.ReceiveAnyDamage`
  (params (Damage :type "Float (single-precision)") (DamageType :type "DamageType Object Reference") (InstigatedBy :type "Controller Object Reference") (DamageCauser :type "Actor Object Reference"))
  (bind _output_get (set `self.Health` (- (`self.Health`) Damage)))
  (if (< _output_get 0.0)
    (`self.Death`)))

(fn `UserConstructionScript`)